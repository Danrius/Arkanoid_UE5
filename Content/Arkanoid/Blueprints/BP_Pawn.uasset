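; Player paddle pawn for an Arkanoid game, moved sideways by mouse or axis input with sweep.
; It spawns a ball on its socket and uses bound death events to deduct lives, respawn and trigger game over, which banks earned money.
; Overlapped BP_Bonus pickups switch by type to paddle, ball or life effects, with retriggerable delays reverting timed ones.
; Extra balls each add a life and are tracked in an array.
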(event `InputAxis|MouseMove`
  (params (AxisValue :type "Float (single-precision)"))
  ;[1 1 1] Pawn Movement
  (`self.K2_AddActorWorldOffset` (`KismetMathLibrary.MakeVector` 0.0 (* AxisValue (`self.Pawn Speed Mouse`))) true))

(event `InputAxis|Move`
  (params (AxisValue :type "Float (single-precision)"))
  ;[1 1 1] Pawn Movement
  (`self.K2_AddActorWorldOffset` (`KismetMathLibrary.MakeVector` 0.0 (* AxisValue (`GameplayStatics.GetWorldDeltaSeconds`) (`self.Pawn Speed`))) true))

(event `self.ReceiveBeginPlay`
  ;[1 1 1] Begin Play
  (bind _asbp_game_instance (cast `/Game/Arkanoid/Blueprints/BP_GameInstance` (`GameplayStatics.GetGameInstance`)))
  (set `self.Game Instance` _asbp_game_instance)
  (`self.Spawn Ball`))

(event `Spawn Ball`
  (bind (_returnvalue_location _returnvalue_rotation) (`KismetMathLibrary.BreakTransform` (`SceneComponent.GetSocketTransform` (`self.StaticMesh`) "Ball" "RTS_World")))
  ;[1 1 1] Spawn Ball
  (if (== (`self.Lives`) 0)
    (`self.Game Over`)
    (else
      (`self.Alive Ball`
        (:`then`)
        (:`else`
          (if (`KismetArrayLibrary.Array_IsEmpty` (`self.All Extra Balls`))
            (bind _returnvalue (`|SpawnActorFromClass` "/Game/Arkanoid/Blueprints/BP_Ball.BP_Ball_C" (`KismetMathLibrary.MakeTransform` _returnvalue_location _returnvalue_rotation) "AlwaysSpawn" "OverrideRootScale" null null))
            (bind _output_get (set `self.Alive Ball` _returnvalue))
            (`self.K2_AttachToComponent` _output_get (`self.StaticMesh`) "Ball" "SnapToTarget" "SnapToTarget" "SnapToTarget" true)
            (add `/Game/Arkanoid/Blueprints/BP_Ball.Ball Dead` (`self.Alive Ball`) (delegate `Sphere Dead`))))))))

(event `Sphere Dead`
  ;[1 1 1] Spawn Ball
  (if (== (`self.Lives`) 0)
    (`self.Game Over`)
    (else
      (set `self.Lives` (- (`self.Lives`) 1))
      (`GameplayStatics.PlaySound2D` "/Game/Arkanoid/Audio/Celtic_Multimedia_Wrong.Celtic_Multimedia_Wrong" 1.0 1.0 0.0 null null)
      (`GameplayStatics.PlayWorldCameraShake` "/Game/Arkanoid/Blueprints/BP_CameraShake.BP_CameraShake_C" (0.0 0.0 0.0) 0.0 3000.0)
      (`KismetSystemLibrary.Delay` 0.2)
      (`self.Spawn Ball`))))

(event `Game Over`
  ;[1 1 1] Game Over
  (`GameplayStatics.PlaySound2D` "/Game/Arkanoid/Audio/Celtic_Fantasy_05.Celtic_Fantasy_05" 1.0 1.0 0.0 null null)
  (`GameplayStatics.SetGamePaused` true)
  (set `/Game/Arkanoid/Blueprints/BP_GameInstance.Money` (+ (`/Game/Arkanoid/Blueprints/BP_GameInstance.Money` (`self.Game Instance`)) (`self.Earned Money`)) (`self.Game Instance`))
  (`WidgetLayoutLibrary.RemoveAllWidgets`)
  (bind _returnvalue (`|CreateWidget` "/Game/Arkanoid/UI/WG_GameOver.WG_GameOver_C"))
  (bind _output_get (set `self.WG Game Over` _returnvalue))
  (`UserWidget.AddToViewport` _output_get 0)
  (`WidgetBlueprintLibrary.SetInputMode_UIOnlyEx` (`GameplayStatics.GetPlayerController` 0) (`self.WG Game Over`))
  (set `PlayerController.bShowMouseCursor` true (`GameplayStatics.GetPlayerController` 0)))

(event `self.StaticMesh.OnComponentBeginOverlap`
  (params (OverlappedComponent :type "PrimitiveComponent Object Reference") (OtherActor :type "Actor Object Reference") (OtherComp :type "PrimitiveComponent Object Reference") (OtherBodyIndex :type Integer) (bFromSweep :type Boolean) (SweepResult :type "HitResult Structure (by ref)"))
  ;[1 1 1] Bonuses
  (bind _asbp_bonus (cast `/Game/Arkanoid/Blueprints/BP_Bonus` OtherActor))
  (bind _output_get (set `self.Bonus` _asbp_bonus))
  (switch `/Game/Arkanoid/Blueprints/Bonus_Type` (`/Game/Arkanoid/Blueprints/BP_Bonus.Bonus Type` _output_get)
    (:`NewEnumerator0`
      (`self.Expand Pawn`)
      (`GameplayStatics.PlaySound2D` "/Game/Arkanoid/Audio/Celtic_Multimedia_Correct.Celtic_Multimedia_Correct" 1.0 1.0 0.0 null null :!label _label)
      (`self.K2_DestroyActor` (`self.Bonus`)))
    (:`NewEnumerator3`
      (`self.Enlarge Ball`)
      (goto _label))
    (:`NewEnumerator4`
      (`self.Extra Ball`)
      (goto _label))
    (:`NewEnumerator5`
      (`self.Extra Life`)
      (goto _label))
    (:`NewEnumerator7`
      (`self.Shrink Paddle`)
      (`GameplayStatics.PlaySound2D` "/Game/Arkanoid/Audio/Celtic_Multimedia_Wrong.Celtic_Multimedia_Wrong" 1.0 1.0 0.0 null null :!label _label_2)
      (`self.K2_DestroyActor` (`self.Bonus`)))
    (:`NewEnumerator8`
      (`self.Shrink Ball`)
      (goto _label_2))
    (:`NewEnumerator9`
      (`self.Fast Ball`)
      (goto _label_2))
    (:`NewEnumerator10`
      (`self.Life Loss`)
      (goto _label_2))))

(event `Expand Pawn`
  ;[1 1 1] Bonuses
  (`StaticMeshComponent.SetStaticMesh` (`self.StaticMesh`) "/Game/Arkanoid/Assets/Expanded_Pawn.Expanded_Pawn")
  (`KismetSystemLibrary.RetriggerableDelay` 5.0)
  (`StaticMeshComponent.SetStaticMesh` (`self.StaticMesh`) "/Game/Arkanoid/Assets/Pawn.Pawn"))

(event `Enlarge Ball`
  (bind (_relativescale3d_x _relativescale3d_y _relativescale3d_z) (`KismetMathLibrary.BreakVector` (`SceneComponent.RelativeScale3D` (`/Game/Arkanoid/Blueprints/BP_Ball.Ball` (`self.Alive Ball`)))))
  (bind (_relativescale3d_x_2 _relativescale3d_y_2 _relativescale3d_z_2) (`KismetMathLibrary.BreakVector` (`SceneComponent.RelativeScale3D` (`Actor.RootComponent` (`self.Array Element`)))))
  ;[1 1 1] Bonuses
  (if (`KismetArrayLibrary.Array_IsEmpty` (`self.All Extra Balls`))
    (`self.Alive Ball` :!label _label_3
      (:`then`
        (`SceneComponent.SetRelativeScale3D` (`/Game/Arkanoid/Blueprints/BP_Ball.Ball` (`self.Alive Ball`)) (1.4 1.4 1.4))
        (`KismetSystemLibrary.RetriggerableDelay` 5.0)
        (`self.Alive Ball`
          (:`then`
            (if (and (> _relativescale3d_x 1.0) (> _relativescale3d_y 1.0) (> _relativescale3d_z 1.0))
              (`SceneComponent.SetRelativeScale3D` (`/Game/Arkanoid/Blueprints/BP_Ball.Ball` (`self.Alive Ball`)) (1.0 1.0 1.0))))
          (:`else`)))
      (:`else`))
    (else
      (`|ExecutionSequence`
        (:`then_0`
          (goto _label_3))
        (:`then_1`
          (for _array_element (`self.All Extra Balls`)
            (bind _output_get (set `self.Array Element` _array_element))
            (`/Engine/EditorBlueprintResources/StandardMacros.IsValid` _output_get
              (:`Is Valid`
                (`SceneComponent.SetRelativeScale3D` (`Actor.RootComponent` (`self.Array Element`)) (1.4 1.4 1.4)))))
          (`KismetSystemLibrary.RetriggerableDelay` 5.0)
          (for _array_element_2 (`self.All Extra Balls`)
            (`/Engine/EditorBlueprintResources/StandardMacros.IsValid` _array_element_2
              (:`Is Valid`
                (if (and (> _relativescale3d_x_2 1.0) (> _relativescale3d_y_2 1.0) (> _relativescale3d_z_2 1.0))
                  (`SceneComponent.SetRelativeScale3D` (`Actor.RootComponent` (`self.Array Element`)) (1.0 1.0 1.0)))))))))))

(event `Extra Ball`
  (bind (_returnvalue_location _returnvalue_rotation) (`KismetMathLibrary.BreakTransform` (`SceneComponent.GetSocketTransform` (`self.StaticMesh`) "Ball" "RTS_World")))
  ;[1 1 1] Bonuses
  (set `self.Lives` (+ (`self.Lives`) 1))
  (bind _returnvalue (`|SpawnActorFromClass` "/Game/Arkanoid/Blueprints/BP_ExtraBall.BP_ExtraBall_C" (`KismetMathLibrary.MakeTransform` _returnvalue_location _returnvalue_rotation) "AdjustIfPossibleButAlwaysSpawn" "OverrideRootScale" null null))
  (bind _output_get (set `self.Alive Extra Ball` _returnvalue))
  (`KismetArrayLibrary.Array_Add` (`self.All Extra Balls`) _output_get)
  (add `/Game/Arkanoid/Blueprints/BP_ExtraBall.Extra Sphere Dead` (`self.Alive Extra Ball`) (delegate `Extra Sphere Dead`)))

(event `Extra Sphere Dead`
  ;[1 1 1] Bonuses
  (`KismetArrayLibrary.Array_Resize` (`self.All Extra Balls`) (- (`KismetArrayLibrary.Array_Length` (`self.All Extra Balls`)) 1))
  (if (not (== (`self.Lives`) 0))
    (set `self.Lives` (- (`self.Lives`) 1))
    (`GameplayStatics.PlaySound2D` "/Game/Arkanoid/Audio/Celtic_Multimedia_Wrong.Celtic_Multimedia_Wrong" 1.0 1.0 0.0 null null)
    (`GameplayStatics.PlayWorldCameraShake` "/Game/Arkanoid/Blueprints/BP_CameraShake.BP_CameraShake_C" (0.0 0.0 0.0) 0.0 3000.0)
    (`KismetSystemLibrary.Delay` 0.2)
    (`self.Spawn Ball`)))

(event `Extra Life`
  ;[1 1 1] Bonuses
  (set `self.Lives` (+ (`self.Lives`) 1))
  (bind _returnvalue (`|CreateWidget` "/Game/Arkanoid/UI/WG_ExtraLife.WG_ExtraLife_C"))
  (`UserWidget.AddToViewport` _returnvalue 0))

(event `Shrink Paddle`
  ;[1 1 1] Bonuses
  (`StaticMeshComponent.SetStaticMesh` (`self.StaticMesh`) "/Game/Arkanoid/Assets/Shrinked_Pawn.Shrinked_Pawn")
  (`KismetSystemLibrary.RetriggerableDelay` 5.0)
  (`StaticMeshComponent.SetStaticMesh` (`self.StaticMesh`) "/Game/Arkanoid/Assets/Pawn.Pawn"))

(event `Shrink Ball`
  (bind (_relativescale3d_x _relativescale3d_y _relativescale3d_z) (`KismetMathLibrary.BreakVector` (`SceneComponent.RelativeScale3D` (`Actor.RootComponent` (`self.Array Element`)))))
  (bind (_relativescale3d_x_2 _relativescale3d_y_2 _relativescale3d_z_2) (`KismetMathLibrary.BreakVector` (`SceneComponent.RelativeScale3D` (`/Game/Arkanoid/Blueprints/BP_Ball.Ball` (`self.Alive Ball`)))))
  ;[1 1 1] Bonuses
  (if (`KismetArrayLibrary.Array_IsEmpty` (`self.All Extra Balls`))
    (`self.Alive Ball` :!label _label_4
      (:`then`
        (`SceneComponent.SetRelativeScale3D` (`/Game/Arkanoid/Blueprints/BP_Ball.Ball` (`self.Alive Ball`)) (0.6 0.6 0.6))
        (`KismetSystemLibrary.RetriggerableDelay` 5.0)
        (`self.Alive Ball`
          (:`then`
            (if (and (< _relativescale3d_x_2 1.0) (< _relativescale3d_y_2 1.0) (< _relativescale3d_z_2 1.0))
              (`SceneComponent.SetRelativeScale3D` (`/Game/Arkanoid/Blueprints/BP_Ball.Ball` (`self.Alive Ball`)) (1.0 1.0 1.0))))
          (:`else`)))
      (:`else`))
    (else
      (`|ExecutionSequence`
        (:`then_0`
          (goto _label_4))
        (:`then_1`
          (for _array_element (`self.All Extra Balls`)
            (bind _output_get (set `self.Array Element` _array_element))
            (`/Engine/EditorBlueprintResources/StandardMacros.IsValid` _output_get
              (:`Is Valid`
                (`SceneComponent.SetRelativeScale3D` (`Actor.RootComponent` (`self.Array Element`)) (0.6 0.6 0.6)))))
          (`KismetSystemLibrary.RetriggerableDelay` 5.0)
          (for _array_element_2 (`self.All Extra Balls`)
            (`/Engine/EditorBlueprintResources/StandardMacros.IsValid` _array_element_2
              (:`Is Valid`
                (if (and (< _relativescale3d_x 1.0) (< _relativescale3d_y 1.0) (< _relativescale3d_z 1.0))
                  (`SceneComponent.SetRelativeScale3D` (`Actor.RootComponent` (`self.Array Element`)) (1.0 1.0 1.0)))))))))))

(event `Fast Ball`
  ;[1 1 1] Bonuses
  (if (`KismetArrayLibrary.Array_IsEmpty` (`self.All Extra Balls`))
    (`self.Alive Ball` :!label _label_5
      (:`then`
        (set `/Game/Arkanoid/Blueprints/BP_Ball.Speed` 30.0 (`self.Alive Ball`))
        (`KismetSystemLibrary.RetriggerableDelay` 5.0)
        (`self.Alive Ball`
          (:`then`
            (if (> (`/Game/Arkanoid/Blueprints/BP_Ball.Speed` (`self.Alive Ball`)) 20.0)
              (set `/Game/Arkanoid/Blueprints/BP_Ball.Speed` 20.0 (`self.Alive Ball`))))
          (:`else`)))
      (:`else`))
    (else
      (`|ExecutionSequence`
        (:`then_0`
          (goto _label_5))
        (:`then_1`
          (for _array_element (`self.All Extra Balls`)
            (bind _output_get (set `self.Array Element` _array_element))
            (`/Engine/EditorBlueprintResources/StandardMacros.IsValid` _output_get
              (:`Is Valid`
                (set `/Game/Arkanoid/Blueprints/BP_ExtraBall.Speed` 30.0 (`self.Array Element`)))))
          (`KismetSystemLibrary.RetriggerableDelay` 5.0)
          (for _array_element_2 (`self.All Extra Balls`)
            (`/Engine/EditorBlueprintResources/StandardMacros.IsValid` _array_element_2
              (:`Is Valid`
                (if (> (`/Game/Arkanoid/Blueprints/BP_ExtraBall.Speed` (`self.Array Element`)) 20.0)
                  (set `/Game/Arkanoid/Blueprints/BP_ExtraBall.Speed` 20.0 (`self.Array Element`)))))))))))

(event `Life Loss`
  ;[1 1 1] Bonuses
  (set `self.Lives` (- (`self.Lives`) 1))
  (bind _returnvalue (`|CreateWidget` "/Game/Arkanoid/UI/WG_LifeLoss.WG_LifeLoss_C"))
  (`UserWidget.AddToViewport` _returnvalue 0)
  (if (== (`self.Lives`) 0)
    (`self.Game Over`)))

(fn `UserConstructionScript`)