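; BP_Block is a breakable Arkanoid block that starts with random health from one to three.
; Each hit lowers health and swaps the mesh material to show what remains.
; The final hit has a weighted chance to spawn BP_Bonus, credits the player pawn's EarnedMoney with the starting health, broadcasts BlockDead and plays a sound.
; It then destroys only the hit component, leaving the actor flagged IsDead.
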(event `self.ReceiveHit`
  (params (MyComp :type "PrimitiveComponent Object Reference") (Other :type "Actor Object Reference") (OtherComp :type "PrimitiveComponent Object Reference") (bSelfMoved :type Boolean) (HitLocation :type "Vector Structure") (HitNormal :type "Vector Structure") (NormalImpulse :type "Vector Structure") (Hit :type "HitResult Structure (by ref)"))
  (bind (_returnvalue_x _returnvalue_y) (`KismetMathLibrary.BreakVector` (`SceneComponent.K2_GetComponentLocation` (`self.Component`))))
  (set `self.Component` MyComp)
  (if (== (`self.Health`) 1)
    (if (`KismetMathLibrary.RandomBoolWithWeight` 0.3)
      (`|SpawnActorFromClass` "/Game/Arkanoid/Blueprints/BP_Bonus.BP_Bonus_C" (`KismetMathLibrary.MakeTransform` (`KismetMathLibrary.MakeVector` _returnvalue_x _returnvalue_y 100.0)) "AlwaysSpawn" "OverrideRootScale" null null))
    (`|ExecutionSequence`
      (:`then_0`
        (bind _asbp_pawn (cast `/Game/Arkanoid/Blueprints/BP_Pawn` (`GameplayStatics.GetPlayerPawn` 0)))
        (bind _output_get (set `self.BP Pawn` _asbp_pawn))
        (set `/Game/Arkanoid/Blueprints/BP_Pawn.Earned Money` (+ (`/Game/Arkanoid/Blueprints/BP_Pawn.Earned Money` _output_get) (`self.Default Health`)) (`self.BP Pawn`)))
      (:`then_1`
        (set `self.Is Dead` true)
        (`self.Block Dead`))
      (:`then_2`
        (`GameplayStatics.PlaySound2D` "/Game/Arkanoid/Audio/WoodHit_BW_18513.WoodHit_BW_18513" 1.0 1.0 0.0 null null))
      (:`then_3`
        (`ActorComponent.K2_DestroyComponent` (`self.Component`))))
    (else
      (set `self.Health` (- (`self.Health`) 1))
      (switch `int` (stale `self.ReceiveBeginPlay` _output_get_2) :!label _label
        (:`1`
          (`PrimitiveComponent.SetMaterial` (`self.StaticMesh`) 0 "/Game/Arkanoid/Materials/MTL_Block1.MTL_Block1"))
        (:`2`
          (`PrimitiveComponent.SetMaterial` (`self.StaticMesh`) 0 "/Game/Arkanoid/Materials/MTL_Block2.MTL_Block2"))
        (:`3`
          (`PrimitiveComponent.SetMaterial` (`self.StaticMesh`) 0 "/Game/Arkanoid/Materials/MTL_Block3.MTL_Block3"))))))

(event `self.ReceiveBeginPlay`
  (bind _output_get (set `self.Default Health` (`KismetMathLibrary.RandomIntegerInRange` 1 3)))
  (bind _output_get_2 (set `self.Health` _output_get))
  (goto _label))

(fn `UserConstructionScript`)