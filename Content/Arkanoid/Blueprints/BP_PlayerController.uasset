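; Player controller for the Arkanoid game that toggles the pause menu from the Pause input action.
; It lazily creates and caches a WG_Pause widget on first use.
; Each press flips the game's paused state, adding the widget to the viewport with Game and UI input focused on it, or removing it and restoring game-only input.
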(event `InputAction|Pause` :paused true
  (params (Key :type "Key Structure"))
  (:`Pressed`
    (`/Engine/EditorBlueprintResources/StandardMacros.IsValid` (`self.WG Pause`)
      (:`Is Valid`
        _)
      (:`Is Not Valid`
        (bind _returnvalue (`|CreateWidget` "/Game/Arkanoid/UI/WG_Pause.WG_Pause_C"))
        (set `self.WG Pause` _returnvalue)))
    (if (`GameplayStatics.IsGamePaused`)
      (`GameplayStatics.SetGamePaused` false)
      (`Widget.RemoveFromParent` (`self.WG Pause`))
      (`WidgetBlueprintLibrary.SetInputMode_GameOnly` (`GameplayStatics.GetPlayerController` 0))
      (else
        (`GameplayStatics.SetGamePaused` true)
        (`UserWidget.AddToViewport` (`self.WG Pause`) 0)
        (`WidgetBlueprintLibrary.SetInputMode_GameAndUIEx` (`GameplayStatics.GetPlayerController` 0) (`self.WG Pause`))))))

(fn `UserConstructionScript`)