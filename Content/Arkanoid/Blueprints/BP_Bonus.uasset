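; Arkanoid bonus pickup that moves through the level as one of several power-ups or penalties.
; The construction script rolls a random BonusType from 1 to 7, so option 0 (ExpandPaddle) is never picked.
; The type sets the mesh: BonusBall for helpful effects, SpikyBall for harmful ones.
; Tick moves it along Direction at Speed without sweep, and overlapping a KillZVolume destroys it.
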(event `self.ReceiveActorBeginOverlap`
  (params (OtherActor :type "Actor Object Reference"))
  (cast `KillZVolume` OtherActor)
  (`self.K2_DestroyActor`))

(event `self.ReceiveTick`
  (params (DeltaSeconds :type "Float (single-precision)"))
  (`self.K2_AddActorWorldOffset` (* DeltaSeconds (`self.Speed`) (`self.Direction`))))

(fn `UserConstructionScript`
  (bind _output_get (set `self.Bonus Type` (select `int` (`KismetMathLibrary.RandomIntegerInRange` 1 7) :`0` "NewEnumerator0" :`1` "NewEnumerator3" :`2` "NewEnumerator4" :`3` "NewEnumerator5" :`4` "NewEnumerator7" :`5` "NewEnumerator8" :`6` "NewEnumerator9" :`7` "NewEnumerator10" :!type "/Game/Arkanoid/Blueprints/Bonus_Type Enum")))
  (switch `/Game/Arkanoid/Blueprints/Bonus_Type` _output_get
    (:`NewEnumerator0`
      (`StaticMeshComponent.SetStaticMesh` (`self.StaticMesh`) "/Game/Arkanoid/Assets/BonusBall.BonusBall" :!label _label))
    (:`NewEnumerator3`
      (goto _label))
    (:`NewEnumerator4`
      (goto _label))
    (:`NewEnumerator5`
      (goto _label))
    (:`NewEnumerator7`
      (`StaticMeshComponent.SetStaticMesh` (`self.StaticMesh`) "/Game/Arkanoid/Assets/SpikyBall.SpikyBall" :!label _label_2))
    (:`NewEnumerator8`
      (goto _label_2))
    (:`NewEnumerator9`
      (goto _label_2))
    (:`NewEnumerator10`
      (goto _label_2))))