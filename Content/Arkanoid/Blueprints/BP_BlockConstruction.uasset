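; Arkanoid block field that spawns each level's blocks and detects when the player has cleared them.
; The construction script lays out an X-by-Y grid of box components as spawn points.
; BeginPlay fills each point with either an occasional indestructible block or a randomly rotated BP_Block bound to BlockDead.
; When all BP_Blocks are dead, it plays a sound, awards the pawn money and a level, then reruns the spawn loop after a delay.
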(event `self.ReceiveBeginPlay`
  (for _array_element (`self.Collision Array`) :!label _label
    (if (`KismetMathLibrary.RandomBoolWithWeight` 0.1)
      (bind (_returnvalue_x _returnvalue_y) (`KismetMathLibrary.BreakVector` (`SceneComponent.K2_GetComponentLocation` _array_element)))
      (`|SpawnActorFromClass` "/Game/Arkanoid/Blueprints/BP_IndestructibleBlock.BP_IndestructibleBlock_C" (`KismetMathLibrary.MakeTransform` (`KismetMathLibrary.MakeVector` _returnvalue_x _returnvalue_y 60.0) (struct) (2.4 2.4 2.4)) "AlwaysSpawn" "SelectDefaultAtRuntime" null null)
      (else
        (bind _returnvalue (`|SpawnActorFromClass` "/Game/Arkanoid/Blueprints/BP_Block.BP_Block_C" (`KismetMathLibrary.MakeTransform` (`SceneComponent.K2_GetComponentLocation` _array_element) (struct) (2.5 2.5 2.5)) "AlwaysSpawn" "SelectDefaultAtRuntime" null null))
        (set `self.Block` _returnvalue)
        (`|ExecutionSequence`
          (:`then_0`
            (bind _output_get (set `self.Block Rotation` (select `int` (`KismetMathLibrary.RandomIntegerInRange` 0 3) :`0` "NewEnumerator0" :`1` "NewEnumerator1" :`2` "NewEnumerator2" :`3` "NewEnumerator3" :!type "/Game/Arkanoid/Blueprints/Block_Rotation Enum")))
            (switch `/Game/Arkanoid/Blueprints/Block_Rotation` _output_get
              (:`NewEnumerator0`
                (`SceneComponent.K2_SetRelativeRotation` :`self` (`Actor.RootComponent` (`self.Block`))))
              (:`NewEnumerator1`
                (`SceneComponent.K2_SetRelativeRotation` (`Actor.RootComponent` (`self.Block`)) (struct :`Yaw` 90.0) false false))
              (:`NewEnumerator2`
                (`SceneComponent.K2_SetRelativeRotation` (`Actor.RootComponent` (`self.Block`)) (struct :`Yaw` -90.0) false false))
              (:`NewEnumerator3`
                (`SceneComponent.K2_SetRelativeRotation` (`Actor.RootComponent` (`self.Block`)) (struct :`Yaw` -180.0) false false))))
          (:`then_1`
            (add `/Game/Arkanoid/Blueprints/BP_Block.Block Dead` (`self.Block`) (delegate `Block Dead`))))))))

(event `Block Dead`
  (set `self.Are All Dead?` true)
  (bind _outactors (`GameplayStatics.GetAllActorsOfClass` "/Game/Arkanoid/Blueprints/BP_Block.BP_Block_C"))
  (for _array_element _outactors
    (if (not (`/Game/Arkanoid/Blueprints/BP_Block.Is Dead` _array_element))
      (set `self.Are All Dead?` false)
      (break)))
  (if (`self.Are All Dead?`)
    (`GameplayStatics.PlaySound2D` "/Game/Arkanoid/Audio/Celtic_Multimedia_Approve.Celtic_Multimedia_Approve" 1.0 1.0 0.0 null null)
    (bind _asbp_pawn (cast `/Game/Arkanoid/Blueprints/BP_Pawn` (`GameplayStatics.GetPlayerPawn` 0)))
    (bind _output_get (set `self.Pawn` _asbp_pawn))
    (set `/Game/Arkanoid/Blueprints/BP_Pawn.Earned Money` (+ (`/Game/Arkanoid/Blueprints/BP_Pawn.Earned Money` _output_get) 50) (`self.Pawn`))
    (`/Engine/EditorBlueprintResources/StandardMacros.IncrementInt` (`/Game/Arkanoid/Blueprints/BP_Pawn.Level` (`self.Pawn`))
      (:`  `
        (`KismetSystemLibrary.Delay` 0.5)
        (goto _label)))))

(fn `UserConstructionScript`
  (for _index (range (`self.Y`))
    (for _index_2 (range (`self.X`))
      (bind _returnvalue (`AddComponent|NODE_AddBoxComponent-1` :`RelativeTransform` (`KismetMathLibrary.MakeTransform` (`KismetMathLibrary.MakeVector` (`KismetMathLibrary.Conv_IntToDouble` (* _index_2 (`self.Padding`))) (`KismetMathLibrary.Conv_IntToDouble` (* _index (`self.Padding`)))) (struct) (1.5 1.5 1.5))))
      (`KismetArrayLibrary.Array_Add` (`self.Collision Array`) _returnvalue))))