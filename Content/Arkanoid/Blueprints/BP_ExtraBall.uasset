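; BP_ExtraBall is an extra ball for an Arkanoid game that bounces around until it reaches a kill volume.
; BeginPlay sets a forward direction with random sideways spread, and Tick moves the ball by swept local offsets on the XY plane.
; Blocking hits reflect the direction off the surface normal, while Hit events play a wood impact sound.
; Overlapping a KillZVolume broadcasts ExtraSphereDead, then destroys the ball.
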(event `self.ReceiveActorBeginOverlap`
  (params (OtherActor :type "Actor Object Reference"))
  (cast `KillZVolume` OtherActor)
  (`self.Extra Sphere Dead`)
  (`self.K2_DestroyActor`))

(event `self.ReceiveTick`
  (params (DeltaSeconds :type "Float (single-precision)"))
  (bind (_returnvalue_x _returnvalue_y) (`KismetMathLibrary.BreakVector` (* (* (`self.Direction`) (`self.Speed`)) DeltaSeconds)))
  (bind _sweephitresult (`self.K2_AddActorLocalOffset` (`KismetMathLibrary.MakeVector` _returnvalue_x _returnvalue_y) true))
  (bind (_bblockinghit _binitialoverlap _time _distance _location _impactpoint _normal) (`GameplayStatics.BreakHitResult` _sweephitresult))
  (if _bblockinghit
    (bind (_returnvalue_x_2 _returnvalue_y_2) (`KismetMathLibrary.BreakVector` (`KismetMathLibrary.GetReflectionVector` (`self.Direction`) _normal)))
    (set `self.Direction` (`KismetMathLibrary.MakeVector` _returnvalue_x_2 _returnvalue_y_2))))

(event `self.ReceiveBeginPlay`
  (set `self.Direction` (`KismetMathLibrary.MakeVector` 100.0 (`KismetMathLibrary.RandomFloatInRange` -50.0 50.0))))

(event `self.ReceiveHit`
  (params (MyComp :type "PrimitiveComponent Object Reference") (Other :type "Actor Object Reference") (OtherComp :type "PrimitiveComponent Object Reference") (bSelfMoved :type Boolean) (HitLocation :type "Vector Structure") (HitNormal :type "Vector Structure") (NormalImpulse :type "Vector Structure") (Hit :type "HitResult Structure (by ref)"))
  (`GameplayStatics.PlaySound2D` "/Game/Arkanoid/Audio/Wood_Hit_Single.Wood_Hit_Single" 1.0 1.0 0.0 null null))

(fn `UserConstructionScript`)